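; AI controller for Nox NPC characters that drives patrolling and enemy detection through a behavior tree.
; On BeginPlay it runs NPC_BehaviorTree, caches the controlled NPC and seeds the blackboard with its patrol path looping, forward direction and wait time.
; Perception updates on any NoxCharacter set CanSeeEnemy from whether it was sensed, and print a debug message even when sight is lost.
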(event OnTargetPerceptionUpdated(AIPerception)
  (params (Actor :type Actor%20Object%20Reference) (Stimulus :type AI%20Stimulus%20Structure))
  (Utilities|Casting|CastToNoxCharacter Actor)
  (AI|Components|Blackboard|SetValueasBool (AI|GetBlackboard 0) (Utilities|Name|MakeLiteralName "CanSeeEnemy") (.bSuccessfullySensed (Utilities|Struct|BreakAIStimulus Stimulus)))
  (Development|PrintString "I SEE YOU"))

(event EventBeginPlay
  (AI|RunBehaviorTree "/Game/ContentNox/Character/NPC/NPC_BehaviorTree.NPC_BehaviorTree")
  (bind _asnox_character_npc_bp (Utilities|Casting|CastToNoxCharacter_NPC_BP (Pawn|GetControlledPawn)))
  (bind _output_get (Variables|Default|SetControlledCharacter_NPC _asnox_character_npc_bp))
  (AI|Components|Blackboard|SetValueasBool (AI|GetBlackboard 0) (Utilities|Name|MakeLiteralName "PatrolPathLooping") (Variables|/Game/ContentNox/Character/NPC/Tools/PatrollPath.PatrollPath_C|GetShouldLoop (Variables|/Game/ContentNox/Character/NPC/NoxCharacter_NPC_BP.NoxCharacter_NPC_BP_C|GetPatrolPath _output_get)))
  (AI|Components|Blackboard|SetValueasBool (AI|GetBlackboard 0) (Utilities|Name|MakeLiteralName "PatrolDirection") true)
  (AI|Components|Blackboard|SetValueasFloat (AI|GetBlackboard 0) (Utilities|Name|MakeLiteralName "WaitTime") (Variables|/Game/ContentNox/Character/NPC/Tools/PatrollPath.PatrollPath_C|GetWaitTime (Variables|/Game/ContentNox/Character/NPC/NoxCharacter_NPC_BP.NoxCharacter_NPC_BP_C|GetPatrolPath (Variables|Default|GetControlledCharacter_NPC)))))

(event EventTick
  (params (DeltaSeconds :type Float%20%28single-precision%29)))

(fn ConstructionScript)